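; Player character Blueprint for a hero who switches between earth, ice and fire forms by swapping skeletal meshes, with camera, movement and launch-based jump input.
; Ability inputs branch on form when grounded and idle: ice fires spikes, earth spawns a wall, fire briefly boosts speed; ability B is empty.
; Earth's wall sets animation flags and disables input until EndAttackingVar restores control.
; Movement-driven time dilation is present but disconnected.
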(event Custom|EndAttacking%20Var
  ;[1 1 1] End Attacking Variable (recieve from Anim BP)
  (Input|EnableInput 0)
  (Utilities|FlowControl|Delay 0.8)
  (Variables|Default|SetAttackActive? false))

(event EventBeginPlay)

(event EventTick
  (params (DeltaSeconds :type Float%20%28single-precision%29))
  ;[1 1 1] Not sure if this feature fits the gameplay we have in mind?
  ;;[1 1 1] Time manipulation feature and checking if the values have changed to determine whether time should speed up or slow down
  ;;;[1 1 1] Update functiion similiar to Unity
)

(event Input|ActionEvents|InputActionPlayerJump
  (params (Key :type Key%20Structure))
  ;[1 1 1] Flappy bird Jumping feature in progress
  (:Pressed
    (if (not (AI|Components|NavMovement|IsFalling (Variables|Character|GetCharacterMovement)))
      (Character|LaunchCharacter "0, 0,1800.000000" false true))))

(event Input|ActionEvents|InputActionSwitch_Earth
  (params (Key :type Key%20Structure))
  ;[1 1 1] Dpeneding on element mode change the mesh
  (:Pressed
    (Utilities|FlowControl|Delay 1.0)
    (Variables|Default|SetForm 0)
    (Class|SkinnedMeshComponent|SetSkeletalMesh (Variables|Character|GetMesh) "/Game/Sasha/Character/Asset_Character_Dwayne_RockForm.Asset_Character_Dwayne_RockForm" true)))

(event Input|ActionEvents|InputActionSwitch_Fire
  (params (Key :type Key%20Structure))
  ;[1 1 1] Dpeneding on element mode change the mesh
  (:Pressed
    (Utilities|FlowControl|Delay 1.0)
    (Variables|Default|SetForm 2)
    (Class|SkinnedMeshComponent|SetSkeletalMesh (Variables|Character|GetMesh) "/Game/Sasha/Character/Dwayne_Fire2.Dwayne_Fire2" true)))

(event Input|ActionEvents|InputActionPlayerAbility_C
  (params (Key :type Key%20Structure))
  (bind _returnvalue (Transformation|GetActorRotation))
  (bind _charactermovement (Variables|Character|GetCharacterMovement))
  ;[1 1 1] Activate Ability & switch based on form
  (:Pressed
    (if (not (or (Variables|Default|GetAttackActive?) (AI|Components|NavMovement|IsFalling (Variables|Character|GetCharacterMovement))))
      (switch int (Variables|Default|GetForm)
        (:0
          ;[1 1 1] RockCTemp (Will make a wall) (T to activate)
          (CallFunction|AbilityRockCFunction)
          (Utilities|FlowControl|Delay 0.15)
          (Game|SpawnActorfromClass "/Game/Blueprints/EarthWall.EarthWall_C" (Math|Transform|MakeTransform (+ (Transformation|GetActorLocation) (* (Math|Vector|GetForwardVector _returnvalue) 2.5e+02)) _returnvalue) "Undefined" 0 0)
          (Variables|Default|SetRockCActive false))
        (:2
          (Variables|/Script/Engine.CharacterMovementComponent|SetMaxWalkSpeed _charactermovement 2e+03)
          (Variables|/Script/Engine.CharacterMovementComponent|SetMaxAcceleration _charactermovement 5e+03)
          (Utilities|FlowControl|Delay 2.0)
          (Variables|/Script/Engine.CharacterMovementComponent|SetMaxWalkSpeed _charactermovement 8e+02)
          (Variables|/Script/Engine.CharacterMovementComponent|SetMaxAcceleration _charactermovement 2048.0))))))

(event Input|ActionEvents|InputActionPlayerAbility_B
  (params (Key :type Key%20Structure))
  ;[1 1 1] Activate Ability & switch based on form
  (:Pressed
    (if (not (or (Variables|Default|GetAttackActive?) (AI|Components|NavMovement|IsFalling (Variables|Character|GetCharacterMovement))))
      (switch int (Variables|Default|GetForm)))))

(event Input|ActionEvents|InputActionPlayerAbility_A
  (params (Key :type Key%20Structure))
  (bind _returnvalue (Pawn|GetControlRotation :!class /Script/Engine.Pawn))
  ;[1 1 1] Activate Ability & switch based on form
  (:Pressed
    (if (not (or (Variables|Default|GetAttackActive?) (AI|Components|NavMovement|IsFalling (Variables|Character|GetCharacterMovement))))
      (switch int (Variables|Default|GetForm)
        (:1
          ;[1 1 1] Ice_Projectile
          (Game|SpawnActorfromClass "/Game/Blueprints/Spikes.Spikes_C" (Math|Transform|MakeTransform (+ (Transformation|GetActorLocation) (* (Math|Vector|GetForwardVector _returnvalue) 2e+02)) _returnvalue) "Undefined" 0 0))))))

(event Input|ActionEvents|InputActionSwitch_Ice
  (params (Key :type Key%20Structure))
  ;[1 1 1] Dpeneding on element mode change the mesh
  (:Pressed
    (Utilities|FlowControl|Delay 1.0)
    (Variables|Default|SetForm 1)
    (Class|SkinnedMeshComponent|SetSkeletalMesh (Variables|Character|GetMesh) "/Game/Sasha/Character/Dwayne_Ice4.Dwayne_Ice4" true)))

(event Input|AxisEvents|InputAxisLookRight
  (params (AxisValue :type Float%20%28single-precision%29))
  ;[0 1 0.03281] Basic Camera
  (Pawn|Input|AddControllerYawInput AxisValue))

(event Input|AxisEvents|InputAxisLookUp
  (params (AxisValue :type Float%20%28single-precision%29))
  ;[0 1 0.03281] Basic Camera
  (Pawn|Input|AddControllerPitchInput AxisValue))

(event Input|AxisEvents|InputAxisMoveForBack
  (params (AxisValue :type Float%20%28single-precision%29))
  ;[1 1 1] Player Manipulation and Animation BP
  (Pawn|Input|AddMovementInput (Math|Vector|GetForwardVector (Math|Rotator|MakeRotator 0.0 0.0 (.Yaw (Math|Rotator|BreakRotator (Pawn|GetControlRotation :!class /Script/Engine.Pawn))))) AxisValue false)
  ;[1 1 1] Values for storing -1 or +1 for movement for time manipulation
  (Variables|Default|SetHAxis AxisValue))

(event Input|AxisEvents|InputAxisMoveLefRigh
  (params (AxisValue :type Float%20%28single-precision%29))
  ;[1 1 1] Player Manipulation and Animation BP
  (Pawn|Input|AddMovementInput (Math|Vector|GetRightVector (Math|Rotator|MakeRotator 0.0 0.0 (.Yaw (Math|Rotator|BreakRotator (Pawn|GetControlRotation :!class /Script/Engine.Pawn))))) AxisValue false)
  ;[1 1 1] Values for storing -1 or +1 for movement for time manipulation
  (Variables|Default|SetVAxis AxisValue))

(fn ConstructionScript)

(fn AbilityRockCFunction
  (Variables|Default|SetRockCActive true)
  (Variables|Default|SetAttackActive? true)
  (Input|DisableInput 0))

(fn AbilityIceBFunction
  (Variables|Default|SetIceBActive true)
  (Variables|Default|SetAttackActive? false))

(fn AbilityRockBFunction
  (Variables|Default|SetRockBActive true)
  (Variables|Default|SetAttackActive? true))